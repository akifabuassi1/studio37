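; Aximmetry tracked camera actor that renders three video billboards (BA, BB, BC) in the Unreal scene, driven by Aximmetry control data.
; Each tick updates the camera and projects the video onto each billboard's main, reflection, shadow and depth components.
; Reflection method and ray tracing cvars select which components render reflections.
; Clip-plane scene captures merge into an RGB mask sent back to Aximmetry, and an HDR control switches the output device.
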(event `self.ReceiveBeginPlay`
  (`parent.ReceiveBeginPlay`)
  (`/Game/Aximmetry_TrackedCam_3-Bill/Blueprints/Components/Camera.BeginPlay` (`self.Camera`) self)
  (`self.InitializeMaskCapture` (`self.BA Mask Capture`))
  (`self.InitializeMaskCapture` (`self.BB Mask Capture`))
  (`self.InitializeMaskCapture` (`self.BC Mask Capture`))
  (`/Game/Aximmetry_TrackedCam_3-Bill/Blueprints/Components/Color_Merger.BeginPlay` (`self.MaskMerger`))
  (add `AximmetryTrigger.Trigger` (`AximmetryFunctionLibrary.GetAximmetryTrigger` "Control Data:Camera Cut" 504) (delegate `OnCameraCut`))
  (bind _returnvalue (`KismetSystemLibrary.GetConsoleVariableIntValue` "r.ReflectionMethod"))
  (set `self.ReflectionMethod` _returnvalue)
  (bind _returnvalue_2 (`KismetSystemLibrary.GetConsoleVariableBoolValue` "r.RayTracing.Shadows"))
  (set `self.RayTracingShadows` _returnvalue_2)
  (bind _returnvalue_3 (`KismetSystemLibrary.GetConsoleVariableBoolValue` "r.Lumen.HardwareRayTracing"))
  (set `self.Lumen Hardware Ray Tracing` _returnvalue_3)
  (bind _returnvalue_4 (`KismetSystemLibrary.GetConsoleVariableIntValue` "r.Lumen.HardwareRayTracing.LightingMode"))
  (set `self.Lumen Hardware Ray Tracing Lighting Mode` _returnvalue_4)
  (bind _returnvalue_5 (`KismetSystemLibrary.GetConsoleVariableIntValue` "r.HDR.Display.OutputDevice"))
  (set `self.OriginalOutputDevice` _returnvalue_5)
  (`KismetSystemLibrary.ExecuteConsoleCommand` "r.HDR.Display.OutputDevice 0" null))

(event `OnCameraCut`
  (`PlayerCameraManager.SetGameCameraCutThisFrame` (`GameplayStatics.GetPlayerCameraManager` 0))
  (set `SceneCaptureComponent2D.bCameraCutThisFrame` true (`self.BA Mask Capture`))
  (set `SceneCaptureComponent2D.bCameraCutThisFrame` true (`self.BB Mask Capture`))
  (set `SceneCaptureComponent2D.bCameraCutThisFrame` true (`self.BC Mask Capture`)))

(event `self.ReceiveEndPlay`
  (params (EndPlayReason :type "EEndPlayReason Enum" :default "Destroyed"))
  (`KismetSystemLibrary.ExecuteConsoleCommand` (`KismetStringLibrary.Concat_StrStr` "r.HDR.Display.OutputDevice " (`KismetStringLibrary.Conv_IntToString` (`self.OriginalOutputDevice`))) null))

(event `self.ReceiveTick`
  (params (DeltaSeconds :type "Float (single-precision)"))
  (bind _returnvalue (`AximmetryFunctionLibrary.GetAximmetryLogical` "Control Data:B Mask" 506 true))
  (bind _returnvalue_2 (`AximmetryFunctionLibrary.GetAximmetryScalar` "Control Data:Projection FOV" 502 90.0))
  (bind (_returnvalue_x _returnvalue_y) (`KismetMathLibrary.BreakVector` (`AximmetryFunctionLibrary.GetAximmetryVector` "Out Size")))
  (bind _returnvalue_3 (`AximmetryFunctionLibrary.GetAximmetryLogical` "Control Data:Virtuals" 505 true))
  (bind _returnvalue_4 (`AximmetryFunctionLibrary.GetAximmetryLogical` "Control Data:Tracked Cam Active" 523))
  (bind _returnvalue_5 (`KismetMathLibrary.Round` _returnvalue_x))
  (`parent.ReceiveTick` DeltaSeconds)
  (if (< (`self.Prewarm`) 5)
    (`/Engine/EditorBlueprintResources/StandardMacros.IncrementInt` (`self.Prewarm`)
      (:`  `
        (`self.SetActorHiddenInGame` true)
        (bind _returnvalue_6 (`AximmetryFunctionLibrary.GetAximmetryVideo` "B Texture" 507 false true "TA_Clamp" :!label _label))
        (bind _returnvalue_7 (`AximmetryFunctionLibrary.GetAximmetryVideo` "B Refl Texture" 508 false true "TA_Clamp"))
        (bind _returnvalue_8 (`AximmetryFunctionLibrary.GetAximmetryVideo` "B Shadow Texture" 509 false false "TA_Clamp"))
        (`self.UpdateBillboard` (`self.BA Billboard`) (`self.BA Reflection`) (`self.BA Shadow`) (`self.BA Depth`) (`self.BA Mask Capture`) (`AximmetryFunctionLibrary.GetAximmetryLogical` "Control Data:BA/Active" 611) _returnvalue_3 _returnvalue (`AximmetryFunctionLibrary.GetAximmetryLogical` "Control Data:BA/Lit" 616) (`AximmetryFunctionLibrary.GetAximmetryLogical` "Control Data:BA/Cast Shadow" 617 true) (`AximmetryFunctionLibrary.GetAximmetryLogical` "Control Data:BA/Render To Depth" 618 true) (`AximmetryFunctionLibrary.GetAximmetryLogical` "Control Data:BA/Inverse Tonemap" 620 true) (`AximmetryFunctionLibrary.GetAximmetryTransformation` "Control Data:BA/Transform" 612) (`AximmetryFunctionLibrary.GetAximmetryTransformation` "Control Data:BA/Refl Transform" 614) (`AximmetryFunctionLibrary.GetAximmetryTransformation` "Control Data:BA/Shadow Transform" 615) (`AximmetryFunctionLibrary.GetAximmetryTransformation` "Control Data:BA/Proj Transform" 613) _returnvalue_2 _returnvalue_6 _returnvalue_7 _returnvalue_8 (`AximmetryFunctionLibrary.GetAximmetryScalar` "Control Data:BA/Shadow Depth" 621 20.0) (`AximmetryFunctionLibrary.GetAximmetryTransformation` "Control Data:BA/Shadow Projection Transform" 622) (`AximmetryFunctionLibrary.GetAximmetryLogical` "Control Data:BA/Alpha Correction") (`AximmetryFunctionLibrary.GetAximmetryScalar` "Control Data:BA/Ray Traced Reflection Intensity" 0 1.0))
        (`self.UpdateBillboard` (`self.BB Billboard`) (`self.BB Reflection`) (`self.BB Shadow`) (`self.BB Depth`) (`self.BB Mask Capture`) (`AximmetryFunctionLibrary.GetAximmetryLogical` "Control Data:BB/Active" 711) _returnvalue_3 _returnvalue (`AximmetryFunctionLibrary.GetAximmetryLogical` "Control Data:BB/Lit" 716) (`AximmetryFunctionLibrary.GetAximmetryLogical` "Control Data:BB/Cast Shadow" 717 true) (`AximmetryFunctionLibrary.GetAximmetryLogical` "Control Data:BB/Render To Depth" 718 true) (`AximmetryFunctionLibrary.GetAximmetryLogical` "Control Data:BB/Inverse Tonemap" 720 true) (`AximmetryFunctionLibrary.GetAximmetryTransformation` "Control Data:BB/Transform" 712) (`AximmetryFunctionLibrary.GetAximmetryTransformation` "Control Data:BB/Refl Transform" 714) (`AximmetryFunctionLibrary.GetAximmetryTransformation` "Control Data:BB/Shadow Transform" 715) (`AximmetryFunctionLibrary.GetAximmetryTransformation` "Control Data:BB/Proj Transform" 713) _returnvalue_2 _returnvalue_6 _returnvalue_7 _returnvalue_8 (`AximmetryFunctionLibrary.GetAximmetryScalar` "Control Data:BB/Shadow Depth" 721 20.0) (`AximmetryFunctionLibrary.GetAximmetryTransformation` "Control Data:BB/Shadow Projection Transform" 722) (`AximmetryFunctionLibrary.GetAximmetryLogical` "Control Data:BB/Alpha Correction") (`AximmetryFunctionLibrary.GetAximmetryScalar` "Control Data:BB/Ray Traced Reflection Intensity" 0 1.0))
        (`self.UpdateBillboard` (`self.BC Billboard`) (`self.BC Reflection`) (`self.BC Shadow`) (`self.BC Depth`) (`self.BC Mask Capture`) (`AximmetryFunctionLibrary.GetAximmetryLogical` "Control Data:BC/Active" 811) _returnvalue_3 _returnvalue (`AximmetryFunctionLibrary.GetAximmetryLogical` "Control Data:BC/Lit" 816) (`AximmetryFunctionLibrary.GetAximmetryLogical` "Control Data:BC/Cast Shadow" 817 true) (`AximmetryFunctionLibrary.GetAximmetryLogical` "Control Data:BC/Render To Depth" 818 true) (`AximmetryFunctionLibrary.GetAximmetryLogical` "Control Data:BC/Inverse Tonemap" 820 true) (`AximmetryFunctionLibrary.GetAximmetryTransformation` "Control Data:BC/Transform" 812) (`AximmetryFunctionLibrary.GetAximmetryTransformation` "Control Data:BC/Refl Transform" 814) (`AximmetryFunctionLibrary.GetAximmetryTransformation` "Control Data:BC/Shadow Transform" 815) (`AximmetryFunctionLibrary.GetAximmetryTransformation` "Control Data:BC/Proj Transform" 813) _returnvalue_2 _returnvalue_6 _returnvalue_7 _returnvalue_8 (`AximmetryFunctionLibrary.GetAximmetryScalar` "Control Data:BC/Shadow Depth" 821 20.0) (`AximmetryFunctionLibrary.GetAximmetryTransformation` "Control Data:BC/Shadow Projection Transform" 822) (`AximmetryFunctionLibrary.GetAximmetryLogical` "Control Data:BC/Alpha Correction") (`AximmetryFunctionLibrary.GetAximmetryScalar` "Control Data:BC/Ray Traced Reflection Intensity" 0 1.0))
        (bind _merged (`/Game/Aximmetry_TrackedCam_3-Bill/Blueprints/Components/Color_Merger.Tick` (`self.MaskMerger`) (`SceneCaptureComponent2D.TextureTarget` (`self.BA Mask Capture`)) (`SceneCaptureComponent2D.TextureTarget` (`self.BB Mask Capture`)) (`SceneCaptureComponent2D.TextureTarget` (`self.BC Mask Capture`))))
        (`AximmetryFunctionLibrary.SetAximmetryVideo` "B Mask" 900 "NoColorSpace" false _merged)))
    (else
      (if (and (not (`self.Active`)) _returnvalue_4)
        (`/Game/Aximmetry_TrackedCam_3-Bill/Blueprints/Components/Camera.BeginPlay` (`self.Camera`) self))
      (bind _output_get (set `self.Active` _returnvalue_4))
      (`self.SetActorHiddenInGame` (not _output_get))
      (if _output_get
        (if (!= _returnvalue_5 0)
          (`self.UpdateHDR` (`AximmetryFunctionLibrary.GetAximmetryLogical` "Control Data:HDR"))
          (`/Game/Aximmetry_TrackedCam_3-Bill/Blueprints/Components/Camera.Tick` (`self.Camera`) (`AximmetryFunctionLibrary.GetAximmetryScalar` "Control Data:Cam FOV" 502 90.0) (`AximmetryFunctionLibrary.GetAximmetryScalar` "Control Data:Cam Focus" 503 20.0) (/ (`KismetMathLibrary.Conv_IntToDouble` _returnvalue_5) (`KismetMathLibrary.Conv_IntToDouble` (`KismetMathLibrary.Round` _returnvalue_y))) (`AximmetryFunctionLibrary.GetAximmetryTransformation` "Control Data:Cam Transform" 501))
          (goto _label))))))

(fn `CalcolatePositionOffset`
  (params (From :type "Transform Structure (by ref)") (To :type "Transform Structure (by ref)"))
  (returns (Offset :type "Vector Structure"))
  (return (- (`KismetMathLibrary.TransformLocation` To) (`KismetMathLibrary.TransformLocation` From))))

(fn `CalculateScreenSpaceUVShaderParameters`
  (params (`Projection Transform` :type "Transform Structure (by ref)") (`Projection FOV` :type "Float (double-precision)"))
  (returns (ScreenSpaceUVShaderParameters :type "/Game/Aximmetry_TrackedCam_3-Bill/Blueprints/Components/ScreenSpaceUVParameters Structure"))
  (bind (_x _y _z) (`KismetMathLibrary.Matrix_GetUnitAxes` (`KismetMathLibrary.Conv_TransformToMatrix` `Projection Transform`)))
  (return (make `/Game/Aximmetry_TrackedCam_3-Bill/Blueprints/Components/ScreenSpaceUVParameters` (`KismetMathLibrary.Conv_VectorToLinearColor` (`KismetMathLibrary.TransformLocation` `Projection Transform`)) (`KismetMathLibrary.Conv_VectorToLinearColor` _x) (`KismetMathLibrary.Conv_VectorToLinearColor` _y) (`KismetMathLibrary.Conv_VectorToLinearColor` _z) (* (make `LinearColor` 1.0 (/ 1.0 (`CameraComponent.AspectRatio` (`self.Camera`)))) (`KismetMathLibrary.DegTan` (/ `Projection FOV` 2.0))))))

(fn `InitializeMaskCapture`
  (params (SceneCapture :type "SceneCaptureComponent2D Object Reference"))
  (set `SceneCaptureComponent2D.bUseCustomProjectionMatrix` true SceneCapture)
  (set `SceneCaptureComponent2D.bEnableClipPlane` true SceneCapture)
  ;[1 1 1] Hide the reflection components from the masks (the rest of the components are not visible by default)
  (set `SceneCaptureComponent.HiddenActors` (`|MakeArray` self :!type "Actor Object Reference") SceneCapture)
  (set `SceneCaptureComponent.bCaptureEveryFrame` false SceneCapture)
  (set `SceneCaptureComponent.bCaptureOnMovement` false SceneCapture)
  (set `SceneCaptureComponent.bAlwaysPersistRenderingState` true SceneCapture)
  (set `SceneCaptureComponent.CaptureSource` "SCS_FinalColorLDR" SceneCapture)
  (setmembers `PostProcessSettings` :`StructRef` (`SceneCaptureComponent2D.PostProcessSettings` SceneCapture) :`WeightedBlendables` (make `WeightedBlendables` (`|MakeArray` (make `WeightedBlendable` 1.0 "/Game/Aximmetry_TrackedCam_3-Bill/Materials/Alpha.Alpha") (make `WeightedBlendable` 1.0 "/Game/Aximmetry_TrackedCam_3-Bill/Materials/Empty_Tonemapper.Empty_Tonemapper"))))
  (set `SceneCaptureComponent2D.bForceTemporalJitter` true SceneCapture))

(fn `SelectReflectionTexture`
  (params (Reflection :type "Texture Object Reference") (Billboard :type "Texture Object Reference"))
  (returns (Selected :type "Texture Object Reference"))
  (bind _astexture_render_target_2d (cast `TextureRenderTarget2D` Reflection)
    (:`then`
      (return (select `bool` (and (== (`TextureRenderTarget2D.SizeX` _astexture_render_target_2d) 4) (== (`TextureRenderTarget2D.SizeY` _astexture_render_target_2d) 4)) :`false` Reflection :`true` Billboard)))
    (:`CastFailed`
      (return Billboard))))

(fn `UpdateBillboard`
  (params (BillboardComponent :type "/Game/Aximmetry_TrackedCam_3-Bill/Blueprints/Components/Billboard Object Reference") (ReflectionComponent :type "/Game/Aximmetry_TrackedCam_3-Bill/Blueprints/Components/Reflection Object Reference") (ShadowComponent :type "/Game/Aximmetry_TrackedCam_3-Bill/Blueprints/Components/Shadow Object Reference") (DepthComponent :type "/Game/Aximmetry_TrackedCam_3-Bill/Blueprints/Components/Depth Object Reference") (BillboardMaskCaptureComponent :type "SceneCaptureComponent2D Object Reference") (Active :type Boolean) (Virtuals :type Boolean) (Mask :type Boolean) (Lit :type Boolean) (CastShadow :type Boolean) (EnableScreenSpaceReflections :type Boolean) (InverseTonemap :type Boolean) (BillboardTransform :type "Transform Structure") (ReflectionTransform :type "Transform Structure") (ShadowTransform :type "Transform Structure") (ProjectionTransform :type "Transform Structure (by ref)") (ProjectionFOV :type "Float (double-precision)") (BillboardTexture :type "Texture Object Reference") (BillboardReflectionTexture :type "Texture Object Reference") (BillboardShadowTexture :type "Texture Object Reference") (ShadowDepth :type "Float (double-precision)") (ShadowProjectionTransform :type "Transform Structure (by ref)") (`Alpha Correction` :type Boolean) (RayTracedReflectionIntensity :type "Float (single-precision)"))
  (locals (ReflectionComponentRendersPlanarReflections :type Boolean) (DepthComponentRendersScreenSpaceReflections :type Boolean) (DepthComponentRendersRayTracedReflections :type Boolean) (ShadowComponentRendersRayTracedReflections :type Boolean))
  (bind _screenspaceuvshaderparameters (`self.CalculateScreenSpaceUVShaderParameters` ProjectionTransform ProjectionFOV))
  (bind _reflectionmethod (`self.ReflectionMethod`))
  (bind _raytracingshadows (`self.RayTracingShadows`))
  (bind _returnvalue (and InverseTonemap (not (`self.HDR`))))
  (bind _returnvalue_2 (or (and (== (`self.ReflectionMethod`) 1) (`self.Lumen Hardware Ray Tracing`) (== (`self.Lumen Hardware Ray Tracing Lighting Mode`) 2)) (== (`self.ReflectionMethod`) 3)))
  (`|ExecutionSequence`
    (:`then_0`
      (if EnableScreenSpaceReflections
        (if CastShadow
          (if _raytracingshadows
            (switch `int` _reflectionmethod
              (:`0`
                (set `local.ReflectionComponentRendersPlanarReflections` true)
                (set `local.DepthComponentRendersScreenSpaceReflections` false)
                (set `local.DepthComponentRendersRayTracedReflections` false)
                (set `local.ShadowComponentRendersRayTracedReflections` false))
              (:`1`
                (set `local.ReflectionComponentRendersPlanarReflections` false)
                (set `local.DepthComponentRendersScreenSpaceReflections` true)
                (set `local.DepthComponentRendersRayTracedReflections` false)
                (set `local.ShadowComponentRendersRayTracedReflections` true))
              (:`2`
                (set `local.ReflectionComponentRendersPlanarReflections` true)
                (set `local.DepthComponentRendersScreenSpaceReflections` true)
                (set `local.DepthComponentRendersRayTracedReflections` false)
                (set `local.ShadowComponentRendersRayTracedReflections` false))
              (:`3`
                (set `local.ReflectionComponentRendersPlanarReflections` false)
                (set `local.DepthComponentRendersScreenSpaceReflections` false)
                (set `local.DepthComponentRendersRayTracedReflections` false)
                (set `local.ShadowComponentRendersRayTracedReflections` true)))
            (else
              (switch `int` _reflectionmethod :!label _label
                (:`0`
                  (set `local.ReflectionComponentRendersPlanarReflections` true)
                  (set `local.DepthComponentRendersScreenSpaceReflections` false)
                  (set `local.DepthComponentRendersRayTracedReflections` false)
                  (set `local.ShadowComponentRendersRayTracedReflections` false))
                (:`1`
                  (set `local.ReflectionComponentRendersPlanarReflections` false)
                  (set `local.DepthComponentRendersScreenSpaceReflections` true)
                  (set `local.DepthComponentRendersRayTracedReflections` true)
                  (set `local.ShadowComponentRendersRayTracedReflections` false))
                (:`2`
                  (set `local.ReflectionComponentRendersPlanarReflections` true)
                  (set `local.DepthComponentRendersScreenSpaceReflections` true)
                  (set `local.DepthComponentRendersRayTracedReflections` false)
                  (set `local.ShadowComponentRendersRayTracedReflections` false))
                (:`3`
                  (set `local.ReflectionComponentRendersPlanarReflections` false)
                  (set `local.DepthComponentRendersScreenSpaceReflections` false)
                  (set `local.DepthComponentRendersRayTracedReflections` true)
                  (set `local.ShadowComponentRendersRayTracedReflections` false)))))
          (elif _raytracingshadows
            (goto _label)
            (else
              (goto _label))))
        (elif CastShadow
          (if _raytracingshadows
            (switch `int` _reflectionmethod
              (:`0`
                (set `local.ReflectionComponentRendersPlanarReflections` true)
                (set `local.DepthComponentRendersScreenSpaceReflections` false)
                (set `local.DepthComponentRendersRayTracedReflections` false)
                (set `local.ShadowComponentRendersRayTracedReflections` false))
              (:`1`
                (set `local.ReflectionComponentRendersPlanarReflections` false)
                (set `local.DepthComponentRendersScreenSpaceReflections` false)
                (set `local.DepthComponentRendersRayTracedReflections` false)
                (set `local.ShadowComponentRendersRayTracedReflections` false))
              (:`2`
                (set `local.ReflectionComponentRendersPlanarReflections` true)
                (set `local.DepthComponentRendersScreenSpaceReflections` false)
                (set `local.DepthComponentRendersRayTracedReflections` false)
                (set `local.ShadowComponentRendersRayTracedReflections` false))
              (:`3`
                (set `local.ReflectionComponentRendersPlanarReflections` false)
                (set `local.DepthComponentRendersScreenSpaceReflections` false)
                (set `local.DepthComponentRendersRayTracedReflections` false)
                (set `local.ShadowComponentRendersRayTracedReflections` true)))
            (else
              (switch `int` _reflectionmethod :!label _label_2
                (:`0`
                  (set `local.ReflectionComponentRendersPlanarReflections` true)
                  (set `local.DepthComponentRendersScreenSpaceReflections` false)
                  (set `local.DepthComponentRendersRayTracedReflections` false)
                  (set `local.ShadowComponentRendersRayTracedReflections` false))
                (:`1`
                  (set `local.ReflectionComponentRendersPlanarReflections` false)
                  (set `local.DepthComponentRendersScreenSpaceReflections` false)
                  (set `local.DepthComponentRendersRayTracedReflections` false)
                  (set `local.ShadowComponentRendersRayTracedReflections` false))
                (:`2`
                  (set `local.ReflectionComponentRendersPlanarReflections` true)
                  (set `local.DepthComponentRendersScreenSpaceReflections` false)
                  (set `local.DepthComponentRendersRayTracedReflections` false)
                  (set `local.ShadowComponentRendersRayTracedReflections` false))
                (:`3`
                  (set `local.ReflectionComponentRendersPlanarReflections` false)
                  (set `local.DepthComponentRendersScreenSpaceReflections` false)
                  (set `local.DepthComponentRendersRayTracedReflections` true)
                  (set `local.ShadowComponentRendersRayTracedReflections` false)))))
          (elif _raytracingshadows
            (goto _label_2)
            (else
              (goto _label_2))))))
    (:`then_1`
      (`/Game/Aximmetry_TrackedCam_3-Bill/Blueprints/Components/Billboard.Tick` BillboardComponent Active Virtuals Lit _returnvalue BillboardTexture BillboardTransform _screenspaceuvshaderparameters `Alpha Correction`)
      (bind _selected (`self.SelectReflectionTexture` BillboardReflectionTexture BillboardTexture))
      (`/Game/Aximmetry_TrackedCam_3-Bill/Blueprints/Components/Reflection.Tick` ReflectionComponent (and Active (`local.ReflectionComponentRendersPlanarReflections`)) Lit _returnvalue _selected ReflectionTransform _screenspaceuvshaderparameters `Alpha Correction`)
      (`/Game/Aximmetry_TrackedCam_3-Bill/Blueprints/Components/Shadow.Tick` ShadowComponent (and Active (or CastShadow (`local.ShadowComponentRendersRayTracedReflections`))) BillboardTexture BillboardShadowTexture ShadowTransform (`self.CalculateScreenSpaceUVShaderParameters` ShadowProjectionTransform ProjectionFOV) (`self.RayTracingShadows`) ShadowDepth _returnvalue Lit (select `bool` (and (`local.ShadowComponentRendersRayTracedReflections`) _returnvalue_2) :`true` RayTracedReflectionIntensity))
      (`/Game/Aximmetry_TrackedCam_3-Bill/Blueprints/Components/Depth.Tick` DepthComponent (and Active (or (`local.DepthComponentRendersScreenSpaceReflections`) (`local.DepthComponentRendersRayTracedReflections`))) BillboardTexture BillboardTransform _screenspaceuvshaderparameters _returnvalue (`local.DepthComponentRendersRayTracedReflections`) Lit (select `bool` (and _returnvalue_2 (`local.DepthComponentRendersRayTracedReflections`)) :`true` RayTracedReflectionIntensity) (or (== (`self.ReflectionMethod`) 1) (== (`self.ReflectionMethod`) 2)))
      (`self.UpdateMaskCapture` (and Active Mask) BillboardMaskCaptureComponent BillboardTransform))))

(fn `UpdateHDR`
  (params (HDR :type Boolean))
  (bind _output (`|GetArrayItem` (`.Array` (break `WeightedBlendables` (`.WeightedBlendables` (break `PostProcessSettings` (`CameraComponent.PostProcessSettings` (`self.Camera`))))))))
  (if (!= HDR (`self.HDR`))
    (bind _output_get (set `self.HDR` HDR))
    (if _output_get
      (`KismetSystemLibrary.ExecuteConsoleCommand` "r.HDR.Display.OutputDevice 7" null)
      (setmembers `WeightedBlendable` :`StructRef` _output :`Weight` 1.0)
      (bind _returnvalue (`KismetSystemLibrary.GetConsoleVariableIntValue` "r.DefaultBackBufferPixelFormat"))
      (if (!= _returnvalue 3)
        (`KismetSystemLibrary.PrintString` "Error: Wrong Frame Buffer Pixel Format. HDR rendering will not work correctly.  \nPlease set Frame Buffer Pixel Format to \"Float RGBA\" in the Unreal Project Settings." true false (struct :`R` 1.0 :`A` 1.0) 999999.0 "AximmetryHDRPixelFormatError")
        (`AximmetryFunctionLibrary.Log` "Error: Wrong Frame Buffer Pixel Format. HDR rendering will not work correctly.  \nPlease set Frame Buffer Pixel Format to \"Float RGBA\" in the Unreal Project Settings." "Error"))
      (else
        (`KismetSystemLibrary.ExecuteConsoleCommand` "r.HDR.Display.OutputDevice 0" null)
        (setmembers `WeightedBlendable` :`StructRef` _output :`Weight` 0.0)
        (`KismetSystemLibrary.PrintString` "" true false (struct :`R` 1.0 :`A` 1.0) 0.0 "AximmetryHDRPixelFormatError") ; Clear onscreen warning
      ))))

(fn `UpdateMaskCapture`
  (params (Active :type Boolean) (SceneCapture :type "SceneCaptureComponent2D Object Reference") (`Billboard Transform` :type "Transform Structure (by ref)"))
  (locals (NullRenderTarget :type "TextureRenderTarget2D Object Reference"))
  (bind _returnvalue (`KismetMathLibrary.TransformDirection` `Billboard Transform` (0.0 0.0 1.0)))
  (bind (_returnvalue_x _returnvalue_y) (`KismetMathLibrary.BreakVector` (`AximmetryFunctionLibrary.GetAximmetryVector` "Out Size")))
  (bind _texturetarget (`SceneCaptureComponent2D.TextureTarget` SceneCapture))
  (bind _returnvalue_2 (`KismetMathLibrary.Round` _returnvalue_x))
  (bind _returnvalue_3 (`KismetMathLibrary.Round` _returnvalue_y))
  (if Active
    (if (`KismetSystemLibrary.IsValid` _texturetarget)
      (if (or (!= (`TextureRenderTarget2D.SizeX` _texturetarget) _returnvalue_2) (!= (`TextureRenderTarget2D.SizeY` _texturetarget) _returnvalue_3))
        (bind _returnvalue_4 (`KismetRenderingLibrary.CreateRenderTarget2D` _returnvalue_2 _returnvalue_3 "RTF_R16f" :!label _label))
        (set `SceneCaptureComponent2D.TextureTarget` _returnvalue_4 SceneCapture))
      (else
        (goto _label)))
    (bind _desiredview (`CameraComponent.GetCameraView` (`self.Camera`) 0.0))
    (set `SceneCaptureComponent2D.CustomProjectionMatrix` (`.ProjectionMatrix` (`GameplayStatics.GetViewProjectionMatrix` _desiredview)) SceneCapture)
    (set `SceneCaptureComponent2D.ClipPlaneBase` (+ (`KismetMathLibrary.TransformLocation` `Billboard Transform` (0.0 0.0 1.0)) _returnvalue) SceneCapture)
    (set `SceneCaptureComponent2D.ClipPlaneNormal` _returnvalue SceneCapture)
    (`SceneCaptureComponent2D.CaptureScene` SceneCapture)
    (else
      (set `SceneCaptureComponent2D.TextureTarget` null SceneCapture))))

(fn `UserConstructionScript`
  (`parent.UserConstructionScript`))