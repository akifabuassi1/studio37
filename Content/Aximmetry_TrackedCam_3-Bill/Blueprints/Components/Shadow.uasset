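; Shadow component of an Aximmetry tracked-camera billboard setup, which drives the material that renders the billboard's shadow.
; BeginPlay creates a dynamic material instance; an externally called Tick sets visibility and, when active, updates the transform and material parameters.
; Camera basis parameters feed screen-space UVs, alongside depth, lighting and ray-tracing settings.
; The billboard texture substitutes for the shadow texture without positive depth, and tonemapper bypass supplies an inverse tonemap texture.
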(event `self.ReceiveBeginPlay`
  (bind _returnvalue (`self.CreateDynamicMaterialInstance` 0 "/Game/Aximmetry_TrackedCam_3-Bill/Materials/Shaders/Shadow.Shadow"))
  (set `self.Dynamic Material Instance` _returnvalue))

(fn `Tick`
  (params (Active :type Boolean :default true) (BillboardTexture :type "Texture Object Reference") (ShadowTexture :type "Texture Object Reference") (Transform :type "Transform Structure") (ScreenSpaceUVShaderParameters :type "/Game/Aximmetry_TrackedCam_3-Bill/Blueprints/Components/ScreenSpaceUVParameters Structure") (RayTraced :type Boolean) (Depth :type "Float (double-precision)") (BypassTonemapper :type Boolean) (Lit :type Boolean) (RayTracedReflectionIntensity :type "Float (single-precision)"))
  (bind (_cameraposition _camerabasisx _camerabasisy _camerabasisz _aspectcoefficient) (break `/Game/Aximmetry_TrackedCam_3-Bill/Blueprints/Components/ScreenSpaceUVParameters` ScreenSpaceUVShaderParameters))
  (bind _dynamic_material_instance (`self.Dynamic Material Instance`))
  (bind _dynamic_material_instance_2 (`self.Dynamic Material Instance`))
  (`self.SetVisibility` Active)
  (if Active
    (`self.K2_SetWorldTransform` Transform)
    (`MaterialInstanceDynamic.SetTextureParameterValue` (`self.Dynamic Material Instance`) "Texture" BillboardTexture)
    (`MaterialInstanceDynamic.SetTextureParameterValue` _dynamic_material_instance "ShadowTexture" (select `bool` (> Depth 0.0) :`false` BillboardTexture :`true` ShadowTexture))
    (`MaterialInstanceDynamic.SetScalarParameterValue` _dynamic_material_instance "RayTraced" (`KismetMathLibrary.Conv_BoolToDouble` RayTraced))
    (`MaterialInstanceDynamic.SetScalarParameterValue` _dynamic_material_instance "Depth" (* Depth 100.0))
    (`MaterialInstanceDynamic.SetScalarParameterValue` (`self.Dynamic Material Instance`) "Inverse Tonemap" (`KismetMathLibrary.Conv_BoolToDouble` BypassTonemapper))
    (`MaterialInstanceDynamic.SetScalarParameterValue` (`self.Dynamic Material Instance`) "Lit" (`KismetMathLibrary.Conv_BoolToDouble` Lit))
    (`MaterialInstanceDynamic.SetVectorParameterValue` _dynamic_material_instance_2 "CameraPosition" _cameraposition)
    (`MaterialInstanceDynamic.SetVectorParameterValue` _dynamic_material_instance_2 "CameraBasisX" _camerabasisx)
    (`MaterialInstanceDynamic.SetVectorParameterValue` _dynamic_material_instance_2 "CameraBasisY" _camerabasisy)
    (`MaterialInstanceDynamic.SetVectorParameterValue` _dynamic_material_instance_2 "CameraBasisZ" _camerabasisz)
    (`MaterialInstanceDynamic.SetVectorParameterValue` _dynamic_material_instance_2 "AspectCoefficient" _aspectcoefficient)
    (if BypassTonemapper
      (bind (_tonemap _inversetonemap) (`AximmetryFunctionLibrary.GetTonemapTextures`))
      (`MaterialInstanceDynamic.SetTextureParameterValue` (`self.Dynamic Material Instance`) "InverseTonemapTexture" _inversetonemap))
    (`MaterialInstanceDynamic.SetScalarParameterValue` (`self.Dynamic Material Instance`) "RayTracedReflectionIntensity" RayTracedReflectionIntensity)))