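; Reflection component for an Aximmetry tracked-camera billboard, showing a supplied texture through a dynamic instance of the Billboard material created at BeginPlay.
; Its Tick function sets visibility and, while active, applies the world transform and pushes texture, lighting and screen-space UV camera parameters to the material.
; Tonemapper bypass and alpha correction fetch tonemap lookup textures only when enabled, with the forward tonemap texture needed just for alpha correction.
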(event `self.ReceiveBeginPlay`
  (bind _returnvalue (`self.CreateDynamicMaterialInstance` 0 "/Game/Aximmetry_TrackedCam_3-Bill/Materials/Shaders/Billboard.Billboard"))
  (set `self.Dynamic Material Instance` _returnvalue))

(fn `Tick`
  (params (Active :type Boolean :default true) (Lit :type Boolean :default false) (`Bypass Tonemapper` :type Boolean :default true) (Texture :type "Texture Object Reference") (Transform :type "Transform Structure") (ScreenSpaceUVShaderParameters :type "/Game/Aximmetry_TrackedCam_3-Bill/Blueprints/Components/ScreenSpaceUVParameters Structure") (AlphaCorrection :type Boolean))
  (bind (_cameraposition _camerabasisx _camerabasisy _camerabasisz _aspectcoefficient) (break `/Game/Aximmetry_TrackedCam_3-Bill/Blueprints/Components/ScreenSpaceUVParameters` ScreenSpaceUVShaderParameters))
  (bind _dynamic_material_instance (`self.Dynamic Material Instance`))
  (bind _dynamic_material_instance_2 (`self.Dynamic Material Instance`))
  (`self.SetVisibility` Active)
  (if Active
    (`self.K2_SetWorldTransform` Transform)
    (`MaterialInstanceDynamic.SetTextureParameterValue` (`self.Dynamic Material Instance`) "Texture" Texture)
    (`MaterialInstanceDynamic.SetScalarParameterValue` (`self.Dynamic Material Instance`) "Inverse Tonemap" (`KismetMathLibrary.Conv_BoolToDouble` `Bypass Tonemapper`))
    (`MaterialInstanceDynamic.SetScalarParameterValue` (`self.Dynamic Material Instance`) "Lit" (`KismetMathLibrary.Conv_BoolToDouble` Lit))
    (`MaterialInstanceDynamic.SetVectorParameterValue` _dynamic_material_instance_2 "CameraPosition" _cameraposition)
    (`MaterialInstanceDynamic.SetVectorParameterValue` _dynamic_material_instance_2 "CameraBasisX" _camerabasisx)
    (`MaterialInstanceDynamic.SetVectorParameterValue` _dynamic_material_instance_2 "CameraBasisY" _camerabasisy)
    (`MaterialInstanceDynamic.SetVectorParameterValue` _dynamic_material_instance_2 "CameraBasisZ" _camerabasisz)
    (`MaterialInstanceDynamic.SetVectorParameterValue` _dynamic_material_instance_2 "AspectCoefficient" _aspectcoefficient)
    (`MaterialInstanceDynamic.SetScalarParameterValue` (`self.Dynamic Material Instance`) "AlphaCorrection" (`KismetMathLibrary.Conv_BoolToDouble` AlphaCorrection))
    (if (or `Bypass Tonemapper` AlphaCorrection)
      (bind (_tonemap _inversetonemap) (`AximmetryFunctionLibrary.GetTonemapTextures`))
      (`MaterialInstanceDynamic.SetTextureParameterValue` _dynamic_material_instance "InverseTonemapTexture" _inversetonemap)
      (if AlphaCorrection
        (`MaterialInstanceDynamic.SetTextureParameterValue` _dynamic_material_instance "TonemapTexture" _tonemap)))))