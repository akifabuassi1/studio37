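; Billboard component for the Aximmetry tracked camera setup that displays a supplied texture on a mesh at a given world transform.
; BeginPlay creates a dynamic instance of the Billboard material.
; Its Tick function shows it only when Active and Virtuals, then updates transform, texture, lighting flag and camera parameters for screen-space UVs.
; Tonemap bypass and alpha correction feed inverse and forward tonemap textures into the material as needed.
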(event `self.ReceiveBeginPlay`
  (bind _returnvalue (`self.CreateDynamicMaterialInstance` 0 "/Game/Aximmetry_TrackedCam_3-Bill/Materials/Shaders/Billboard.Billboard"))
  (set `self.DynamicMaterialInstance` _returnvalue))

(fn `Tick`
  (params (Active :type Boolean :default true) (Virtuals :type Boolean :default true) (Lit :type Boolean :default false) (`Bypass Tonemapper` :type Boolean :default true) (Texture :type "Texture Object Reference") (Transform :type "Transform Structure") (ScreenSpaceUVShaderParameters :type "/Game/Aximmetry_TrackedCam_3-Bill/Blueprints/Components/ScreenSpaceUVParameters Structure") (AlphaCorrection :type Boolean))
  (bind (_cameraposition _camerabasisx _camerabasisy _camerabasisz _aspectcoefficient) (break `/Game/Aximmetry_TrackedCam_3-Bill/Blueprints/Components/ScreenSpaceUVParameters` ScreenSpaceUVShaderParameters))
  (bind _returnvalue (and Active Virtuals))
  (bind _dynamicmaterialinstance (`self.DynamicMaterialInstance`))
  (`self.SetVisibility` _returnvalue)
  (if _returnvalue
    (`self.K2_SetWorldTransform` Transform)
    (`MaterialInstanceDynamic.SetTextureParameterValue` (`self.DynamicMaterialInstance`) "Texture" Texture)
    (`MaterialInstanceDynamic.SetScalarParameterValue` (`self.DynamicMaterialInstance`) "Inverse Tonemap" (`KismetMathLibrary.Conv_BoolToDouble` `Bypass Tonemapper`))
    (`MaterialInstanceDynamic.SetScalarParameterValue` (`self.DynamicMaterialInstance`) "Lit" (`KismetMathLibrary.Conv_BoolToDouble` Lit))
    (`MaterialInstanceDynamic.SetVectorParameterValue` (`self.DynamicMaterialInstance`) "CameraPosition" _cameraposition)
    (`MaterialInstanceDynamic.SetVectorParameterValue` (`self.DynamicMaterialInstance`) "CameraBasisX" _camerabasisx)
    (`MaterialInstanceDynamic.SetVectorParameterValue` (`self.DynamicMaterialInstance`) "CameraBasisY" _camerabasisy)
    (`MaterialInstanceDynamic.SetVectorParameterValue` (`self.DynamicMaterialInstance`) "CameraBasisZ" _camerabasisz)
    (`MaterialInstanceDynamic.SetVectorParameterValue` (`self.DynamicMaterialInstance`) "AspectCoefficient" _aspectcoefficient)
    (`MaterialInstanceDynamic.SetScalarParameterValue` (`self.DynamicMaterialInstance`) "AlphaCorrection" (`KismetMathLibrary.Conv_BoolToDouble` AlphaCorrection))
    (if (or `Bypass Tonemapper` AlphaCorrection)
      (bind (_tonemap _inversetonemap) (`AximmetryFunctionLibrary.GetTonemapTextures`))
      (`MaterialInstanceDynamic.SetTextureParameterValue` _dynamicmaterialinstance "InverseTonemapTexture" _inversetonemap)
      (if AlphaCorrection
        (`MaterialInstanceDynamic.SetTextureParameterValue` _dynamicmaterialinstance "TonemapTexture" _tonemap)))))